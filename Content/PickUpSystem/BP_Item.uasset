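; BP_Item is a pickup actor in the PickUpSystem that shrinks away and destroys itself when picked up.
; Its construction script applies two configurable meshes to ItemModel and ItemModel2.
; The PickUp event prints a debug string, plays a sound and starts the Shrink timeline, which scales the root from full size toward zero.
; A short Delay chained to the timeline's Update, rather than Finished, triggers DestroyActor.
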(event `/Game/PickUpSystem/BPI_Items.PickUp`
  (`KismetSystemLibrary.PrintString` "ItemPicked")
  (`GameplayStatics.PlaySound2D` "/Game/Sound/411177__silverillusionist__pick-up-item-1.411177__silverillusionist__pick-up-item-1" 1.0 1.0 0.0 null null)
  (bind (_direction _shrinktimeline) (`Timeline|Shrink`)
    (:`Update`
      (`SceneComponent.SetWorldScale3D` (`self.DefaultSceneRoot`) (`KismetMathLibrary.Conv_DoubleToVector` (`KismetMathLibrary.Lerp` 1.0 0.0 _shrinktimeline)))
      (`KismetSystemLibrary.Delay` 0.4)
      (`self.K2_DestroyActor`))))

(fn `UserConstructionScript`
  (`StaticMeshComponent.SetStaticMesh` (`self.ItemModel`) (`self.ItemModelToPlace`))
  (`StaticMeshComponent.SetStaticMesh` (`self.ItemModel2`) (`self.ItemModelToPlace2`)))