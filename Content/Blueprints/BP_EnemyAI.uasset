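; Enemy character that chases the player on sight, punches in melee, and can be killed by stealth takedown or damage.
; Pawn sensing starts an AI move to the player, then a montage and sphere overlap damage Player-tagged actors.
; Sighting also disables stealth attacks on BP_ThirdPersonCharacter for a timed window.
; Moveto, if stealth is allowed, positions the enemy, plays the victim montage and destroys it.
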(event `self.ReceiveTick`
  (params (DeltaSeconds :type "Float (single-precision)"))
  ;[0 0 0 0] Movement Cool Down When Attacking
  (if (not (`self.isSeeingPlayer`))
    (`MovementComponent.StopMovementImmediately` (`self.CharacterMovement`))))

(event `self.PawnSensing.OnSeePawn`
  (params (Pawn :type "Pawn Object Reference"))
  ;[0 0 0 0] Follow player
  (set `self.isSeeingPlayer` true)
  (`self.FollowPlayer`)
  (if true
    (`self.noPlayerStealhAttack`)
    (set `self.canStealthAttack` false)
    (`KismetSystemLibrary.Delay` 10.0)
    (set `self.canStealthAttack` true)
    (`self.yesPlayerStealthAttack`)
    (else
      (set `self.canStealthAttack` true)
      (`self.yesPlayerStealthAttack`))))

(event `FollowPlayer`
  ;[0 0 0 0] Follow player
  (set `self.canAttack` true)
  (if (`self.isSeeingPlayer`)
    (`|AIMoveTo` self (0.0 0.0 0.0) (`GameplayStatics.GetPlayerCharacter` 0) 70.0
      (:`OnSuccess`
        (if (`self.canAttack`)
          (set `self.canAttack` false)
          (bind _returnvalue (`self.PlayAnimMontage` "/Game/Animations/Paired_CounterPunch_PalmStrike_Att_UE5_Montage.Paired_CounterPunch_PalmStrike_Att_UE5_Montage"))
          (bind _outactors (`KismetSystemLibrary.SphereOverlapActors` (`SceneComponent.K2_GetComponentLocation` (`self.Arrow1`)) 100.0 (`self.Object Types`)))
          (for _array_element _outactors
            (if (`self.ActorHasTag` _array_element "Player")
              (`GameplayStatics.ApplyDamage` _array_element 5.0)))
          (`KismetSystemLibrary.Delay` _returnvalue)
          (set `self.canAttack` true))))
    (else
      (set `self.isSeeingPlayer` false))))

(event `Move to`
  (params (Location :type "Vector Structure") (Rotation :type "Rotator Structure"))
  (if (`self.canStealthAttack`)
    (set `self.canAttack` false)
    (`|AIMoveTo` self Location null
      (:`then`
        (bind _returnvalue (`self.PlayAnimMontage` "/Game/Animations/Paired_Knife_Stealth_KidneyAndNeck_Vic_Montage.Paired_Knife_Stealth_KidneyAndNeck_Vic_Montage"))
        (`self.K2_SetActorRotation` Rotation)
        (`self.SetActorEnableCollision` self false)
        (`KismetSystemLibrary.Delay` _returnvalue)
        (`CharacterMovementComponent.DisableMovement` (`self.CharacterMovement`))
        (`self.K2_DestroyActor`)))))

(event `self.ReceiveAnyDamage`
  (params (Damage :type "Float (single-precision)") (DamageType :type "DamageType Object Reference") (InstigatedBy :type "Controller Object Reference") (DamageCauser :type "Actor Object Reference"))
  ;[0 0 0 0] Health system
  (set `self.Health` (- (`self.Health`) Damage))
  (`KismetSystemLibrary.PrintString` (`KismetStringLibrary.Conv_DoubleToString` (`self.Health`)))
  (if (<= (`self.Health`) 0.0)
    (`self.K2_DestroyActor`)))

(fn `noPlayerStealhAttack`
  (bind _asbp_third_person_character (cast `/Game/ThirdPerson/Blueprints/BP_ThirdPersonCharacter` (`GameplayStatics.GetPlayerPawn` 0)))
  (set `/Game/ThirdPerson/Blueprints/BP_ThirdPersonCharacter.canStealthAttackPlayer` false _asbp_third_person_character))

(fn `UserConstructionScript`)

(fn `yesPlayerStealthAttack`
  (bind _asbp_third_person_character (cast `/Game/ThirdPerson/Blueprints/BP_ThirdPersonCharacter` (`GameplayStatics.GetPlayerPawn` 0)))
  (set `/Game/ThirdPerson/Blueprints/BP_ThirdPersonCharacter.canStealthAttackPlayer` true _asbp_third_person_character))